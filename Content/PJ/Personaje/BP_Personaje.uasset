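; Player character for a side-scrolling platformer with a sprite, handling Enhanced Input movement, jump, crouch and quit.
; Movement runs along world X, flipping controller yaw by acceleration direction; crouching also offsets the sprite vertically.
; Walking off a ledge opens a brief coyote-time window via retriggerable delay, during which jump launches the character upward.
; RespawnPersonaje stores the spawn location at BeginPlay unless flying; an interface event tallies and prints coins.
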(event Custom|Respawn%20Personaje
  ;[1 1 1] Respawn del personaje
  (if (not (Class|NavMovementComponent|IsFlying (Variables|Character|GetCharacterMovement)))
    (Variables|Player|SetPlayer%20Spawn (Transformation|GetActorLocation))))

(event Input|EnhancedActionEvents|EnhancedInputActionIA_Agachado
  (params (ActionValue :type Float%20%28double-precision%29) (ElapsedSeconds :type Float%20%28double-precision%29) (TriggeredSeconds :type Float%20%28double-precision%29) (InputAction :type Input%20Action%20Object%20Reference :default "/Game/Inputs/Input/IA_Agachado.IA_Agachado"))
  ;[1 1 1] Agachado
  (:Started
    (Transformation|AddLocalOffset (Variables|Default|GetSprite) "0.000000,0.000000,17.000000" false false)
    (Character|Crouch))
  (:Completed
    (Transformation|AddLocalOffset (Variables|Default|GetSprite) "0.000000,0.000000,-17.000000" false false)
    (Character|UnCrouch)))

(event Input|EnhancedActionEvents|EnhancedInputActionIA_Moverse
  (params (ActionValue :type Float%20%28double-precision%29) (ElapsedSeconds :type Float%20%28double-precision%29) (TriggeredSeconds :type Float%20%28double-precision%29) (InputAction :type Input%20Action%20Object%20Reference :default "/Game/Inputs/Input/IA_Moverse.IA_Moverse"))
  (bind _returnvalue (Pawn|GetController))
  ;[1 1 1] Movimiento
  (Pawn|Input|AddMovementInput "1.000000,0.000000,0.000000" ActionValue false)
  (Math|Float|CompareFloat (.x (Pawn|Components|CharacterMovement|GetCurrentAcceleration (Variables|Character|GetCharacterMovement))) 0.0
    (:>
      (Pawn|SetControlRotation _returnvalue (Math|Rotator|MakeRotator 0.0 0.0 0.0)))
    (:<
      (Pawn|SetControlRotation _returnvalue (Math|Rotator|MakeRotator 0.0 0.0 1.8e+02)))))

(event Input|EnhancedActionEvents|EnhancedInputActionIA_Saltar
  (params (ActionValue :type Float%20%28double-precision%29) (ElapsedSeconds :type Float%20%28double-precision%29) (TriggeredSeconds :type Float%20%28double-precision%29) (InputAction :type Input%20Action%20Object%20Reference :default "/Game/Inputs/Input/IA_Saltar.IA_Saltar"))
  ;[1 1 1] Salto y Doble Salto
  (:Started
    (Character|Jump)
    (if (Variables|Player|GetEsta%20en%20coyote%20time?)
      (Character|LaunchCharacter "0.000000,0.000000,1200.000000" false true)
      (Development|PrintString "salto" true true "(R=0.174093,G=0.086179,B=1.000000,A=1.000000)" 1.0)))
  (:Completed
    (Character|StopJumping)))

(event Input|EnhancedActionEvents|EnhancedInputActionIA_QuitGame
  (params (ActionValue :type Float%20%28double-precision%29) (ElapsedSeconds :type Float%20%28double-precision%29) (TriggeredSeconds :type Float%20%28double-precision%29) (InputAction :type Input%20Action%20Object%20Reference :default "/Game/Inputs/Input/IA_QuitGame.IA_QuitGame"))
  ;[1 1 1] Salir del juego
  (Game|QuitGame 0 "Quit" false))

(event EventBeginPlay
  (bind _asplayer_controller (Utilities|Casting|CastToPlayerController (Pawn|GetController)))
  (Input|AddMappingContext (PlayerController|LocalPlayerSubsystems|GetEnhancedInputLocalPlayerSubsystem _asplayer_controller) "/Game/Inputs/Mapping/IMC_Personaje.IMC_Personaje" 0 "(bIgnoreAllPressedKeysUntilRelease=True,bForceImmediately=False,bNotifyUserSettings=False)")
  (CallFunction|RespawnPersonaje))

(event EventOnWalkingOffLedge
  (params (PreviousFloorImpactNormal :type Vector%20%28by%20ref%29 :default "0, 0, 0") (PreviousFloorContactNormal :type Vector%20%28by%20ref%29 :default "0, 0, 0") (PreviousLocation :type Vector%20%28by%20ref%29 :default "0, 0, 0") (TimeDelta :type Float%20%28single-precision%29))
  ;[1 1 1] CoyoteTime
  (Development|PrintString "coyote on" true true "(R=0.000000,G=1.000000,B=0.079420,A=1.000000)")
  (Variables|Player|SetEsta%20en%20coyote%20time? true)
  (Utilities|FlowControl|RetriggerableDelay 0.4)
  (Development|PrintString "coyote off" true true "(R=1.000000,G=0.008761,B=0.000000,A=1.000000)")
  (Variables|Player|SetEsta%20en%20coyote%20time? false))

(event EventRecolectarMonedas
  (params (Monedas :type Integer))
  ;[1 1 1] BPI recolectar moneda
  (bind _output_get (Variables|Mochila|SetMonedas (+ Monedas (Variables|Mochila|GetMonedas))))
  (Development|PrintString (Utilities|String|Append "Tienes " (Utilities|String|ToString(Integer) _output_get) " monedas") true true "(R=1.000000,G=0.903009,B=0.000000,A=1.000000)" 5.0))

(fn ConstructionScript)